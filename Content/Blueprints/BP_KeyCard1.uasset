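; BP_KeyCard1 is a collectible key card pickup that hovers and spins in the world.
; On BeginPlay it stores its location and plays the Chronologie timeline, whose tracks drive the mesh yaw rotation and a vertical floating offset on the actor.
; On overlap with BP_Player, it calls the player's CollectObject with index 0, then destroys itself.
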(event `self.ReceiveBeginPlay`
  (bind (_actorlocation_x _actorlocation_y _actorlocation_z) (`KismetMathLibrary.BreakVector` (`self.ActorLocation`)))
  (set `self.ActorLocation` (`self.K2_GetActorLocation`))
  (bind (_direction _rotation _flotte) (`Timeline|Chronologie`)
    (:`Update`
      (`SceneComponent.K2_SetWorldRotation` (`self.KeyCard`) (`KismetMathLibrary.MakeRotator` 0.0 0.0 (* _rotation 360.0)) false false)
      (`self.K2_SetActorLocation` (`KismetMathLibrary.MakeVector` _actorlocation_x _actorlocation_y (+ (/ _flotte 1.5) _actorlocation_z))))))

(event `self.ReceiveActorBeginOverlap`
  (params (OtherActor :type "Actor Object Reference"))
  (bind _asbp_player (cast `/Game/Blueprints/BP_Player` OtherActor))
  (`/Game/Blueprints/BP_Player.CollectObject` _asbp_player 0)
  (`self.K2_DestroyActor`))

(fn `UserConstructionScript`)