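; Locked door that destroys itself, plays an unlock sound and prints a message when its keypad fires.
; On BeginPlay it hides the Green component and binds to every BP_KeyPad whose SwitchNumber matches its DoorNumber.
; Overlap plays a refusal sound and message if BP_ThirdPersonCharacter or BP_Player lacks the K2 keycard.
; A BP_ThirdPersonCharacter with the card instead binds a duplicate open event to matching keypads.
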(event `CustomEvent`
  (`self.K2_DestroyActor`)
  (`GameplayStatics.PlaySoundAtLocation` "/Game/Sons/OpenUnlockElectronic.OpenUnlockElectronic" (0.0 0.0 0.0) (struct) 1.0 1.0 0.0 null null null null)
  (`KismetSystemLibrary.PrintString` "Unlocked"))

(event `self.ReceiveBeginPlay`
  (`SceneComponent.SetVisibility` (`self.Green`) false false)
  (bind _outactors (`GameplayStatics.GetAllActorsOfClass` "/Game/Blueprints/BP_KeyPad.BP_KeyPad_C"))
  (for _array_element _outactors
    (if (== (`/Game/Blueprints/BP_KeyPad.SwitchNumber` _array_element) (`self.DoorNumber`))
      (add `/Game/Blueprints/BP_KeyPad.OpenDoor` _array_element (delegate `CustomEvent`)))))

(event `CustomEvent_1`
  (`self.K2_DestroyActor`)
  (`GameplayStatics.PlaySoundAtLocation` "/Game/Sons/OpenUnlockElectronic.OpenUnlockElectronic" (0.0 0.0 0.0) (struct) 1.0 1.0 0.0 null null null null)
  (`KismetSystemLibrary.PrintString` "Unlocked"))

(event `self.ReceiveActorBeginOverlap`
  (params (OtherActor :type "Actor Object Reference"))
  (`|ExecutionSequence`
    (:`then_0`
      (bind _asbp_third_person_character (cast `/Game/ThirdPerson/Blueprints/BP_ThirdPersonCharacter` OtherActor))
      (if (`/Game/ThirdPerson/Blueprints/BP_ThirdPersonCharacter.K2NotCollected` _asbp_third_person_character)
        (`GameplayStatics.PlaySoundAtLocation` "/Game/Sons/RefusedAccess.RefusedAccess" (0.0 0.0 0.0) (struct) 1.0 1.0 0.0 null null null null)
        (`KismetSystemLibrary.PrintString` "The door is locked by a keycard")
        (else
          (bind _outactors (`GameplayStatics.GetAllActorsOfClass` "/Game/Blueprints/BP_KeyPad.BP_KeyPad_C"))
          (for _array_element _outactors
            (if (== (`/Game/Blueprints/BP_KeyPad.SwitchNumber` _array_element) (`self.DoorNumber`))
              (add `/Game/Blueprints/BP_KeyPad.OpenDoor` _array_element (delegate `CustomEvent_1`)))))))
    (:`then_1`
      (bind _asbp_player (cast `/Game/Blueprints/BP_Player` OtherActor))
      (if (`/Game/Blueprints/BP_Player.K2NotCollected` _asbp_player)
        (`GameplayStatics.PlaySoundAtLocation` "/Game/Sons/RefusedAccess.RefusedAccess" (0.0 0.0 0.0) (struct) 1.0 1.0 0.0 null null null null)
        (`KismetSystemLibrary.PrintString` "The door is locked by a keycard")))))

(fn `UserConstructionScript`)