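; Guard AI character that patrols, spots the player and ends the game on catching them.
; On BeginPlay it caches the patrol spline's point count and records in the Blackboard whether a valid path exists.
; PawnSensing stores a seen player as the Blackboard target if none is set, plays a random halt sound and flags chasing.
; While chasing, a CatchCapsule overlap with the player shows the BP_Over widget.
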(event `self.ReceiveBeginPlay`
  (bind _patrolpath (`self.PatrolPath`))
  (bind _returnvalue (`KismetSystemLibrary.IsValid` _patrolpath))
  (if _returnvalue
    (set `self.PatrolPathNodeCount` (`SplineComponent.GetNumberOfSplinePoints` (`/Game/AIPerson/Blueprints/BP_Path.Spline` _patrolpath))))
  (`BlackboardComponent.SetValueAsBool` (`AIBlueprintHelperLibrary.GetBlackboard` null) (`self.Key Name 2`) _returnvalue))

(event `self.PawnSensing.OnSeePawn`
  (params (Pawn :type "Pawn Object Reference"))
  (bind _returnvalue (`AIBlueprintHelperLibrary.GetBlackboard` null))
  (bind _key_name (`self.Key Name`))
  (if (not (`KismetSystemLibrary.IsValid` (`BlackboardComponent.GetValueAsObject` _returnvalue _key_name)))
    (bind _asbp_player (cast `/Game/Blueprints/BP_Player` Pawn))
    (`BlackboardComponent.SetValueAsObject` _returnvalue _key_name _asbp_player)
    (`GameplayStatics.PlaySoundAtLocation` (select `int` (`KismetMathLibrary.RandomInteger` 2) :`0` "/Game/Sons/HALT.HALT" :`1` "/Game/Sons/Halt2.Halt2" :!type "SoundBase Object Reference") (`SceneComponent.K2_GetComponentLocation` (`self.CapsuleComponent`)) (struct) 1.0 1.0 0.0 null null null null)
    (set `self.Chasing` true)))

(event `self.CatchCapsule.OnComponentBeginOverlap`
  (params (OverlappedComponent :type "PrimitiveComponent Object Reference") (OtherActor :type "Actor Object Reference") (OtherComp :type "PrimitiveComponent Object Reference") (OtherBodyIndex :type Integer) (bFromSweep :type Boolean) (SweepResult :type "HitResult Structure (by ref)"))
  (if (`self.Chasing`)
    (cast `/Game/Blueprints/BP_Player` OtherActor)
    (bind _returnvalue (`|CreateWidget` "/Game/UI/BP_Over.BP_Over_C"))
    (`UserWidget.AddToViewport` _returnvalue 0)))

(fn `UserConstructionScript`)