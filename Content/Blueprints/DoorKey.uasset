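; DoorKey is a locked door actor that opens when an overlapping player has collected key K3.
; On overlap, a sequence runs the same check for both BP_ThirdPersonCharacter and BP_Player, reading each one's K3NotCollected flag.
; Without the key it plays a refusal sound and prints a locked message.
; With it, it destroys the Door1 and Box1 components, plays a cell-door sound and prints an unlock message, both sounds playing at world origin.
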(event `self.ReceiveBeginPlay`)

(event `self.ReceiveActorBeginOverlap`
  (params (OtherActor :type "Actor Object Reference"))
  (`|ExecutionSequence`
    (:`then_0`
      (bind _asbp_third_person_character (cast `/Game/ThirdPerson/Blueprints/BP_ThirdPersonCharacter` OtherActor))
      (if (`/Game/ThirdPerson/Blueprints/BP_ThirdPersonCharacter.K3NotCollected` _asbp_third_person_character)
        (`GameplayStatics.PlaySoundAtLocation` "/Game/Sons/RefusedAccess.RefusedAccess" (0.0 0.0 0.0) (struct) 1.0 1.0 0.0 null null null null)
        (`KismetSystemLibrary.PrintString` "The door is locked by a key")
        (else
          (`ActorComponent.K2_DestroyComponent` (`self.Door1`))
          (`ActorComponent.K2_DestroyComponent` (`self.Box1`))
          (`GameplayStatics.PlaySoundAtLocation` "/Game/Sons/prison_cell_door_sound_effect_-_Sky_Sound_Effect__Sound_Effects__Sound_fx__Free_Sound_Effects.prison_cell_door_sound_effect_-_Sky_Sound_Effect__Sound_Effects__Sound_fx__Free_Sound_Effects" (0.0 0.0 0.0) (struct) 1.0 1.0 0.0 null null null null)
          (`KismetSystemLibrary.PrintString` "Door unlock!!!!"))))
    (:`then_1`
      (bind _asbp_player (cast `/Game/Blueprints/BP_Player` OtherActor))
      (if (`/Game/Blueprints/BP_Player.K3NotCollected` _asbp_player)
        (`GameplayStatics.PlaySoundAtLocation` "/Game/Sons/RefusedAccess.RefusedAccess" (0.0 0.0 0.0) (struct) 1.0 1.0 0.0 null null null null)
        (`KismetSystemLibrary.PrintString` "The door is locked by a key")
        (else
          (`ActorComponent.K2_DestroyComponent` (`self.Door1`))
          (`ActorComponent.K2_DestroyComponent` (`self.Box1`))
          (`GameplayStatics.PlaySoundAtLocation` "/Game/Sons/prison_cell_door_sound_effect_-_Sky_Sound_Effect__Sound_Effects__Sound_fx__Free_Sound_Effects.prison_cell_door_sound_effect_-_Sky_Sound_Effect__Sound_Effects__Sound_fx__Free_Sound_Effects" (0.0 0.0 0.0) (struct) 1.0 1.0 0.0 null null null null)
          (`KismetSystemLibrary.PrintString` "Door unlock!!!!"))))))

(fn `UserConstructionScript`)