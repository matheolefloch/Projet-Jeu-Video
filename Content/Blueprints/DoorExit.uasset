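; DoorExit is an exit door actor that stays locked until the overlapping player has collected a keycard.
; On begin overlap, a sequence tries casts to BP_ThirdPersonCharacter and BP_Player, running identical checks on each one's K1NotCollected flag.
; While the flag is set it plays a refusal sound and message; otherwise it destroys itself with an unlock sound and message.
; Both sounds play at the world origin rather than at the door.
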(event `self.ReceiveActorBeginOverlap`
  (params (OtherActor :type "Actor Object Reference"))
  (`|ExecutionSequence`
    (:`then_0`
      (bind _asbp_third_person_character (cast `/Game/ThirdPerson/Blueprints/BP_ThirdPersonCharacter` OtherActor))
      (if (`/Game/ThirdPerson/Blueprints/BP_ThirdPersonCharacter.K1NotCollected` _asbp_third_person_character)
        (`GameplayStatics.PlaySoundAtLocation` "/Game/Sons/RefusedAccess.RefusedAccess" (0.0 0.0 0.0) (struct) 1.0 1.0 0.0 null null null null)
        (`KismetSystemLibrary.PrintString` "The door is locked by a keycard")
        (else
          (`self.K2_DestroyActor`)
          (`GameplayStatics.PlaySoundAtLocation` "/Game/Sons/OpenUnlockElectronic.OpenUnlockElectronic" (0.0 0.0 0.0) (struct) 1.0 1.0 0.0 null null null null)
          (`KismetSystemLibrary.PrintString` "Door unlock!!!!"))))
    (:`then_1`
      (bind _asbp_player (cast `/Game/Blueprints/BP_Player` OtherActor))
      (if (`/Game/Blueprints/BP_Player.K1NotCollected` _asbp_player)
        (`GameplayStatics.PlaySoundAtLocation` "/Game/Sons/RefusedAccess.RefusedAccess" (0.0 0.0 0.0) (struct) 1.0 1.0 0.0 null null null null)
        (`KismetSystemLibrary.PrintString` "The door is locked by a keycard")
        (else
          (`self.K2_DestroyActor`)
          (`GameplayStatics.PlaySoundAtLocation` "/Game/Sons/OpenUnlockElectronic.OpenUnlockElectronic" (0.0 0.0 0.0) (struct) 1.0 1.0 0.0 null null null null)
          (`KismetSystemLibrary.PrintString` "Door unlock!!!!"))))))

(fn `UserConstructionScript`)