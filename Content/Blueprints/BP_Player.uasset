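; Player Blueprint handling axis movement with interpolated turning, plus pickup of two keycards and a key and access to an exit-door keypad.
; Overlap events set per-item flags and print prompts; the door allows code entry only once the second keycard is collected.
; The Collect input closes open pickup popups, collects items with sound and widget, or opens the keypad in UI-only mode.
; A separate event toggles entries in a Collectibles array.
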(event `InputAxis|MoveXAxis`
  (params (AxisValue :type "Float (single-precision)"))
  (`self.AddMovementInput` (10.0 0.0 0.0) AxisValue)
  (if (or (!= (stale `InputAxis|MoveYAxis` AxisValue) 0.0) (!= AxisValue 0.0)) :!label _label
    (`self.K2_SetActorRotation` (`KismetMathLibrary.RInterpTo` (`self.K2_GetActorRotation`) (`KismetMathLibrary.MakeRotator` 0.0 0.0 (+ (`KismetMathLibrary.DegAtan2` (stale `InputAxis|MoveYAxis` AxisValue) AxisValue) -90.0)) (`GameplayStatics.GetWorldDeltaSeconds`) 7.0))))

(event `InputAxis|MoveYAxis`
  (params (AxisValue :type "Float (single-precision)"))
  (`self.AddMovementInput` (0.0 10.0 0.0) AxisValue)
  (goto _label))

(event `CollectObject`
  (params (CollectObject :type Integer))
  (bind _collectibles (`self.Collectibles`))
  (`KismetArrayLibrary.Array_Set` _collectibles CollectObject (not (`|GetArrayItem` _collectibles CollectObject))))

(event `self.ReceiveActorBeginOverlap`
  (params (OtherActor :type "Actor Object Reference"))
  ; To interect with KeycardJerome
  (`|ExecutionSequence`
    (:`then_0`
      (cast `/Game/Blueprints/BP_KeyCardJerome` OtherActor)
      (if (`self.K1NotCollected`)
        (set `self.Keycard` true)
        (`KismetSystemLibrary.PrintString` "Press E to collect Keycard")))
    (:`then_1`
      (cast `/Game/Blueprints/BP_KeyCardJerome2` OtherActor)
      (if (`self.K2NotCollected`)
        (set `self.Keycard2` true)
        (`KismetSystemLibrary.PrintString` "Press E to collect Keycard")))
    (:`then_2`
      (cast `/Game/Blueprints/DoorExitKeyAndCode` OtherActor)
      (if (not (`self.K2NotCollected`))
        (set `self.CanEnterCode` true)
        (`KismetSystemLibrary.PrintString` "Press E to Enter Code")))
    (:`then_3`
      (cast `/Game/Blueprints/BP_KEY` OtherActor)
      (if (`self.K3NotCollected`)
        (set `self.Keycard3` true)
        (`KismetSystemLibrary.PrintString` "Press E to Collect")))))

(event `self.ReceiveActorEndOverlap`
  (params (OtherActor :type "Actor Object Reference"))
  ; To interect with KeycardJerome
  (`|ExecutionSequence`
    (:`then_0`
      (cast `/Game/Blueprints/BP_KeyCardJerome` OtherActor)
      (set `self.Keycard` false))
    (:`then_1`
      (cast `/Game/Blueprints/BP_KeyCardJerome2` OtherActor)
      (set `self.Keycard2` false))
    (:`then_2`
      (cast `/Game/Blueprints/DoorExitKeyAndCode` OtherActor)
      (set `self.CanEnterCode` false))
    (:`then_3`
      (cast `/Game/Blueprints/BP_KEY` OtherActor)
      (set `self.Keycard3` false))))

(event `InputAction|Collect`
  (params (Key :type "Key Structure"))
  (bind _returnvalue (`GameplayStatics.GetPlayerController` 0))
  ; To interect with KeycardJerome
  (:`Pressed`
    (`|ExecutionSequence`
      (:`then_0`
        ; Remove UI from screen when E press and UI active
        (if (`self.UIK3`)
          (set `self.UIK3` false)
          (`Widget.RemoveFromParent` (`self.NewVar_1`))
          (`GameplayStatics.PlaySoundAtLocation` "/Game/Sons/CloseUI.CloseUI" (0.0 0.0 0.0) (struct) 1.0 1.0 0.0 null null null null)))
      (:`then_1`
        (if (`self.UIK2`)
          (set `self.UIK2` false)
          (`Widget.RemoveFromParent` (`self.NewVar_0`))
          (`GameplayStatics.PlaySoundAtLocation` "/Game/Sons/CloseUI.CloseUI" (0.0 0.0 0.0) (struct) 1.0 1.0 0.0 null null null null)))
      (:`then_2`
        (if (`self.UIK1`)
          (set `self.UIK1` false)
          (`Widget.RemoveFromParent` (`self.NewVar`))
          (`GameplayStatics.PlaySoundAtLocation` "/Game/Sons/CloseUI.CloseUI" (0.0 0.0 0.0) (struct) 1.0 1.0 0.0 null null null null)))
      (:`then_3`
        (if (`self.Keycard`)
          (if (`self.K1NotCollected`)
            (`KismetSystemLibrary.PrintString` "Keycard A Collected")
            (set `self.K1NotCollected` false)
            (`GameplayStatics.PlaySoundAtLocation` "/Game/Sons/Collecting.Collecting" (0.0 0.0 0.0) (struct) 1.0 1.0 0.0 null null null null)
            (bind _returnvalue_2 (`|CreateWidget` "/Game/UI/Keycard/UI_PickUpKeyCard.UI_PickUpKeyCard_C"))
            (bind _output_get (set `self.NewVar` _returnvalue_2))
            (`UserWidget.AddToViewport` _output_get 0)
            (set `self.UIK1` true))))
      (:`then_4`
        (if (`self.CanEnterCode`)
          (set `PlayerController.bShowMouseCursor` true _returnvalue)
          (`WidgetBlueprintLibrary.SetInputMode_UIOnlyEx` _returnvalue null)
          (bind _returnvalue_3 (`|CreateWidget` "/Game/UI/Keypad/UIKeypad.UIKeypad_C"))
          (`UserWidget.AddToViewport` _returnvalue_3 0)))
      (:`then_5`
        (if (`self.Keycard2`)
          (if (`self.K2NotCollected`)
            (`KismetSystemLibrary.PrintString` "Keycard A Collected")
            (set `self.K2NotCollected` false)
            (`GameplayStatics.PlaySoundAtLocation` "/Game/Sons/Collecting.Collecting" (0.0 0.0 0.0) (struct) 1.0 1.0 0.0 null null null null)
            (bind _returnvalue_4 (`|CreateWidget` "/Game/UI/Keycard2/UI_PickUpKeyCard2.UI_PickUpKeyCard2_C"))
            (bind _output_get_2 (set `self.NewVar_0` _returnvalue_4))
            (`UserWidget.AddToViewport` _output_get_2 0)
            (set `self.UIK2` true))))
      (:`then_6`
        (if (`self.Keycard3`)
          (if (`self.K3NotCollected`)
            (`KismetSystemLibrary.PrintString` "Key Collected")
            (set `self.K3NotCollected` false)
            (`GameplayStatics.PlaySoundAtLocation` "/Game/Sons/Collecting.Collecting" (0.0 0.0 0.0) (struct) 1.0 1.0 0.0 null null null null)
            (bind _returnvalue_5 (`|CreateWidget` "/Game/UI/Key/UI_PickUpKe.UI_PickUpKe_C"))
            (bind _output_get_3 (set `self.NewVar_1` _returnvalue_5))
            (`UserWidget.AddToViewport` _output_get_3 0)
            (set `self.UIK3` true)))))))

(fn `UserConstructionScript`)